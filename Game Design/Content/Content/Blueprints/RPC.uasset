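; RPC integrates Discord Rich Presence, publishing a status for the game through Init and Shutdown events.
; Init constructs and initializes a DiscordRpc object with an application ID, then sets a hardcoded development status.
; RichPresence writes state, details, start timestamp and image fields into the presence struct and pushes the update, with a second "Rich Presence" function forwarding to it.
; Shutdown clears the presence.
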(event EventInit
  (bind _returnvalue (Game|ConstructObjectfromClass "/Script/DiscordRpc.DiscordRpc"))
  (bind _output_get (Variables|Discord|SetDiscordRPC _returnvalue))
  (Class|DiscordRpc|Initialize _output_get (Variables|Discord|GetApplication%20Id) false)
  (CallFunction|RichPresence "Currently Developing" "Developing"))

(event EventShutdown
  (Class|DiscordRpc|ClearPresence (Variables|Discord|GetDiscordRPC)))

(fn RichPresence
  (params (State :type String) (Details :type String) (Start%20Timestamp :type Integer) (Large%20Image%20Key :type String) (Large%20Image%20Text :type String) (Small%20Image%20Key :type String) (Small%20Image%20Text :type String))
  (bind _discordrpc (Variables|Discord|GetDiscordRPC))
  (bind _structout (Utilities|Struct|SetmembersinDiscordRichPresence (Variables|/Script/DiscordRpc.DiscordRpc|GetRichPresence (Variables|Discord|GetDiscordRPC)) State Details Start%20Timestamp Large%20Image%20Key Large%20Image%20Text Small%20Image%20Key Small%20Image%20Text))
  (Variables|/Script/DiscordRpc.DiscordRpc|SetRichPresence _discordrpc _structout)
  (Class|DiscordRpc|UpdatePresence _discordrpc)
  (return true))

(fn RichPresence
  (params (State :type String) (Details :type String) (Start%20Time :type Integer) (Large%20Image%20Key :type String) (Large%20Image%20Text :type String) (Small%20Image%20Key :type String) (Small%20Image%20Text :type String))
  (Discord|RichPresence State Details Start%20Time Large%20Image%20Key Large%20Image%20Text Small%20Image%20Key Small%20Image%20Text)
  (return false))