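; Door actor that swings open and closed in response to switch activation and deactivation events.
; SwitchActivated plays the DoorActivation timeline, whose DoorPos track drives the Door component's relative yaw, and SwitchDeactivated reverses it.
; Logic for counting active pressure switches against a required number is present but disconnected and unfinished, so the events move the door directly.
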(event Custom|SwitchActivated
  (bind _doorpos (Timeline|DoorActivation Play)
    (:Update
      (Transformation|SetRelativeLocationAndRotation (Variables|Default|GetDoor) "0, 0, 0" (Math|Rotator|MakeRotator 0.0 0.0 _doorpos) false false))))

(event Custom|SwitchDeactivated
  (bind _doorpos (Timeline|DoorActivation Reverse)
    (:Update
      (Transformation|SetRelativeLocationAndRotation (Variables|Default|GetDoor) "0, 0, 0" (Math|Rotator|MakeRotator 0.0 0.0 _doorpos) false false))))

(fn ConstructionScript)