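; Pressure button that sinks when a Cube or BP_ThirdPersonCharacter overlaps it and rises when one leaves.
; BeginPlay caches raised and lowered mesh transforms; separate press and release timelines lerp between them.
; Overlap events handle Cubes directly and forward to custom events for the character, with IsPlayer and IsBox named opposite to those casts.
; Flags never clear, occupants aren't counted, and the sound call is unconnected.
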(event Custom|Event%20ActorEndOverlap%20%28Box%29
  (params (Actor :type Actor%20Object%20Reference))
  (Utilities|Casting|CastToBP_ThirdPersonCharacter Actor)
  (if true
    (Variables|Default|SetisBox true)
    (bind _button_in (Timeline|Timeline ReverseFromEnd)
      (:Update
        (Transformation|SetRelativeTransform (Variables|Default|GetButton%20Mesh) (Math|Transform|Lerp(Transform) (Variables|Default|GetOut%20Position) (Variables|Default|GetIn%20Position) _button_in) false false)))
    (else
      (Variables|Default|SetisBox false))))

(event Custom|Event%20ActorBeginOverlap%20%28Box%29
  (params (OtherActor :type Actor%20Object%20Reference))
  (Utilities|Casting|CastToBP_ThirdPersonCharacter OtherActor)
  (if true
    (Variables|Default|SetisBox true)
    (bind _button_in (Timeline|Button%20In PlayFromStart)
      (:Update
        (Transformation|SetRelativeTransform (Variables|Default|GetButton%20Mesh) (Math|Transform|Lerp(Transform) (Variables|Default|GetOut%20Position) (Variables|Default|GetIn%20Position) _button_in) false false)))
    (else
      (Variables|Default|SetisBox false))))

(event EventBeginPlay
  (bind _button_mesh (Variables|Default|GetButton%20Mesh))
  (bind _returnvalue (Transformation|GetRelativeTransform _button_mesh))
  (Variables|Default|SetOut%20Position (Math|Transform|MakeTransform (.location _returnvalue) (.rotation _returnvalue) (.scale _returnvalue)))
  (Variables|Default|SetIn%20Position (Math|Transform|MakeTransform (- (.location _returnvalue) "0.000000,0.000000,4.000000") (.rotation _returnvalue) (.scale _returnvalue)))
  (Input|EnableInput (Game|GetPlayerController 0)))

(event Collision|EventActorEndOverlap
  (params (OtherActor :type Actor%20Object%20Reference))
  (Utilities|FlowControl|Sequence
    (:then_0
      (Utilities|Casting|CastToCube OtherActor)
      (if true
        (Variables|Default|SetisPlayer true)
        (bind _button_in (Timeline|Timeline ReverseFromEnd)
          (:Update
            (Transformation|SetRelativeTransform (Variables|Default|GetButton%20Mesh) (Math|Transform|Lerp(Transform) (Variables|Default|GetOut%20Position) (Variables|Default|GetIn%20Position) _button_in) false false)))
        (else
          (Variables|Default|SetisPlayer false))))
    (:then_1
      (CallFunction|EventActorEndOverlap(Box) OtherActor))))

(event Collision|EventActorBeginOverlap
  (params (OtherActor :type Actor%20Object%20Reference))
  (Utilities|FlowControl|Sequence
    (:then_0
      (Utilities|Casting|CastToCube OtherActor)
      (if true
        (Variables|Default|SetisPlayer true)
        (bind _button_in (Timeline|Button%20In PlayFromStart)
          (:Update
            (Transformation|SetRelativeTransform (Variables|Default|GetButton%20Mesh) (Math|Transform|Lerp(Transform) (Variables|Default|GetOut%20Position) (Variables|Default|GetIn%20Position) _button_in) false false)))
        (else
          (Variables|Default|SetisPlayer false))))
    (:then_1
      (CallFunction|EventActorBeginOverlap(Box) OtherActor))))

(fn ConstructionScript)