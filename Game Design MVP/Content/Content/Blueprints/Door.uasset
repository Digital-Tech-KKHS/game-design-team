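; Door Blueprint that swings a door's yaw through a timeline, driven by pressure switch events.
; SwitchActivated and SwitchDeactivated raise and lower an active-switch count, then compare it to the number needed.
; While the needed count is at least the active count, activation plays the timeline and deactivation reverses it; otherwise each does the opposite.
; The timeline's DoorPos track sets the door's relative rotation.
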(event Custom|SwitchActivated
  (Math|Integer|IncrementInt (Variables|Default|GetPressureSwitchesActive)
    (:%20%20
      (if (>= (Variables|Default|GetPressureSwitchesNeeded) (Variables|Default|GetPressureSwitchesActive))
        (bind _doorpos (Timeline|DoorActivation Play)
          (:Update
            (Transformation|SetRelativeLocationAndRotation (Variables|Default|GetDoor) "0, 0, 0" (Math|Rotator|MakeRotator 0.0 0.0 _doorpos) false false)))
        (else
          (Timeline|DoorActivation Reverse))))))

(event Custom|SwitchDeactivated
  (Math|Integer|DecrementInt (Variables|Default|GetPressureSwitchesActive)
    (:%20%20
      (if (>= (Variables|Default|GetPressureSwitchesNeeded) (Variables|Default|GetPressureSwitchesActive))
        (bind _doorpos (Timeline|DoorActivation Reverse)
          (:Update
            (Transformation|SetRelativeLocationAndRotation (Variables|Default|GetDoor) "0, 0, 0" (Math|Rotator|MakeRotator 0.0 0.0 _doorpos) false false)))
        (else
          (Timeline|DoorActivation Play))))))

(fn ConstructionScript)